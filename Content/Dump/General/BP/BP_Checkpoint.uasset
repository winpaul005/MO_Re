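; Checkpoint gate that locks the player between two doors to fight a one-time Securitron ambush, or passes them through if their weapon is holstered.
; Entering the trigger closes one door, lights up and spawns delayed enemies at SpawnPoint via the ForEachWithDelay macro.
; Enemies leaving the trigger are untracked; once none remain, the opposite door opens and IsAOen flips to swap door roles for the next pass.
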(event OnComponentBeginOverlap(Tigger)
  (params (OverlappedComponent :type Primitive%20Component%20Object%20Reference) (OtherActor :type Actor%20Object%20Reference) (OtherComp :type Primitive%20Component%20Object%20Reference) (OtherBodyIndex :type Integer) (bFromSweep :type Boolean) (SweepResult :type Hit%20Result%20Structure%20%28by%20ref%29))
  (bind _indoor (Variables|Default|GetInDoor))
  (bind _ausdoor (Variables|Default|GetAusDoor))
  (bind _isaoen (Variables|Default|GetIsAOen))
  (bind _returnvalue (select _isaoen _ausdoor _indoor))
  (bind _relativelocation (Variables|/Script/Engine.SceneComponent|GetRelativeLocation _returnvalue))
  (if (and (== OtherActor (Game|Player|GetPlayerPawn 0)) (not (Variables|Default|GetIsProcessing)))
    (Variables|Default|SetIsProcessing true)
    (Development|PrintString "Let the games begin!")
    (Audio|PlaySound2D "/Game/Dump/General/Audio/SFX/checkpointNewMeat.checkpointNewMeat" 1.0 1.0 0.0 0 0)
    (Rendering|Components|Light|SetIntensity (Variables|Default|GetPointLight) 8e+03)
    (Components|MoveComponentTo _returnvalue (Math|Vector|MakeVector (.x _relativelocation) (.y _relativelocation) (Variables|Default|GetCacheZ)) "0, 0, 0" true true 0.8 false)
    (Utilities|FlowControl|Delay (Variables|Default|GetSpawnStartOffset))
    (bind _returnvalue_2 (Class|CIPlayer|GetIsWeaponHolstred(Message) (Game|Player|GetPlayerPawn 0))) ; Letting player pass checkpoint peacefullt
    (if _returnvalue_2
      (CallFunction|CheckifThatsIt :!label _label)
      (elif (<= (Variables|Default|GetCurrentCreeps) 0)
        (goto _label)
        (else
          (CallFunction|SpawnCreeps))))))

(event OnComponentEndOverlap(Tigger)
  (params (OverlappedComponent :type Primitive%20Component%20Object%20Reference) (OtherActor :type Actor%20Object%20Reference) (OtherComp :type Primitive%20Component%20Object%20Reference) (OtherBodyIndex :type Integer))
  (bind _slaveenemies (Variables|Default|GetslaveEnemies))
  (bind _asbp_securtiron (Utilities|Casting|CastToBP_Securtiron OtherActor))
  (Utilities|Array|RemoveItem _slaveenemies _asbp_securtiron)
  (if (and (<= (Utilities|Array|Length _slaveenemies) 0) (<= (Variables|Default|GetCurrentCreeps) 0))
    (Variables|Default|SetIsProcessing false)
    (CallFunction|CheckifThatsIt)))

(event Custom|CheckIfThatsIt
  (if (not (> (Utilities|Array|Length (Variables|Default|GetslaveEnemies)) 0))
    (Rendering|Components|Light|SetIntensity (Variables|Default|GetPointLight) 0.0)
    (Variables|Default|SetIsProcessing false)
    (Development|PrintString "Checkpoint is clear!")
    (Utilities|FlowControl|Sequence
      (:then_0
        (Components|MoveComponentTo (select (Variables|Default|GetIsAOen) (Variables|Default|GetInDoor) (Variables|Default|GetAusDoor)) (Math|Vector|MakeVector (.x (Variables|/Script/Engine.SceneComponent|GetRelativeLocation (select (Variables|Default|GetIsAOen) (Variables|Default|GetInDoor) (Variables|Default|GetAusDoor)))) (.y (Variables|/Script/Engine.SceneComponent|GetRelativeLocation (select (Variables|Default|GetIsAOen) (Variables|Default|GetInDoor) (Variables|Default|GetAusDoor)))) (+ (.z (Variables|/Script/Engine.SceneComponent|GetRelativeLocation (select (Variables|Default|GetIsAOen) (Variables|Default|GetInDoor) (Variables|Default|GetAusDoor)))) (Variables|Default|GetDoorOffset))) "0, 0, 0" true true 0.8 false)
        (Variables|Default|SetIsCleared true)
        (if (Variables|Default|GetIsAOen)
          (Variables|Default|SetIsAOen false)
          (else
            (Variables|Default|SetIsAOen true)))))))

(event Custom|SpawnCreeps
  (Utilities|ForEachwithDelay 0 (- (Variables|Default|GetMaxCreeps) 1) (Variables|Default|GetCreepSpawnDelay)
    (:Loop%20Body
      (bind _returnvalue (Game|SpawnActorfromClass "/Game/Dump/General/BP/Enemies/BP_Securtiron.BP_Securtiron_C" (Math|Transform|MakeTransform (.OutItem (Utilities|Array|Random (Variables|Default|Getspawnpoints))) "0, 0, 0" "1.000000,1.000000,1.000000") "Undefined" "MultiplyWithRoot" 0 0))
      (Class|CIEntity|ScenarioStartle _returnvalue (Utilities|Array|MakeArray (Game|Player|GetPlayerPawn 0)))
      (Utilities|Array|Add (Variables|Default|GetslaveEnemies) _returnvalue)
      (Variables|Default|SetCurrentCreeps (- (Variables|Default|GetCurrentCreeps) 1))
      (Utilities|FlowControl|Delay (Variables|Default|GetCreepSpawnDelay)))
    (:Completed
      (Variables|Default|SetCurrentCreeps 0))))

(event EventBeginPlay
  (bind _indoor (Variables|Default|GetInDoor))
  (Variables|Default|SetCacheZ (.z (Variables|/Script/Engine.SceneComponent|GetRelativeLocation _indoor)))
  (Transformation|AddRelativeLocation _indoor (Math|Vector|MakeVector 0.0 0.0 (Variables|Default|GetDoorOffset)) false true)
  (Utilities|Array|Add (Variables|Default|Getspawnpoints) (Transformation|GetWorldLocation (Variables|Default|GetSpawnPoint)))
  (Variables|Default|SetCurrentCreeps (Variables|Default|GetMaxCreeps)))

(event Collision|EventActorBeginOverlap
  (params (OtherActor :type Actor%20Object%20Reference)))

(event EventTick
  (params (DeltaSeconds :type Float%20%28single-precision%29)))

(fn ConstructionScript)