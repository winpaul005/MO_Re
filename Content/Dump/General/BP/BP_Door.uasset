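; A door actor that toggles between open and closed when its UseItem event fires.
; A latent MoveComponentTo rotates DefaultSceneRoot over one second to a fixed quarter-turn or back to zero rotation, independent of its starting rotation.
; An IsOpening flag blocks re-triggering during the move, and IsOpen flips once it completes.
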(event EventBeginPlay)

(event Collision|EventActorBeginOverlap
  (params (OtherActor :type Actor%20Object%20Reference)))

(event EventTick
  (params (DeltaSeconds :type Float%20%28single-precision%29)))

(event EventUseItem
  (params (CacheItemID :type Integer) (InventoryC :type C%20Inventory%20Component%20Object%20Reference))
  (bind _defaultsceneroot (Variables|Default|GetDefaultSceneRoot))
  (bind _relativelocation (Variables|/Script/Engine.SceneComponent|GetRelativeLocation _defaultsceneroot))
  (if (Variables|Default|GetIsOpen)
    (if (not (Variables|Default|GetisOpening))
      (Variables|Default|SetisOpening true)
      (Components|MoveComponentTo _defaultsceneroot _relativelocation "0.000000,0.000000,0.000000" false false 1.0 false)
      (Variables|Default|SetisOpening false)
      (Variables|Default|SetIsOpen false))
    (elif (not (Variables|Default|GetisOpening))
      (Variables|Default|SetisOpening true)
      (Components|MoveComponentTo _defaultsceneroot _relativelocation "0.000000,-90.000000,0.000000" false false 1.0 false)
      (Variables|Default|SetisOpening false)
      (Variables|Default|SetIsOpen true))))

(fn ConstructionScript)