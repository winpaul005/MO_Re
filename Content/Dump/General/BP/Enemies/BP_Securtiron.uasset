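; Securitron enemy that shows its AI state on its eye and shoots toward the player when triggered.
; Each tick it copies the IsStartled and IsTriggered blackboard flags into a dynamic eye material.
; While triggered, it fires jittered, debug-drawn hitscan traces at randomized intervals, ignoring Checkpoint-tagged actors and sending PunchMessage to whatever it hits.
; ScenarioProceedTo passes scenario actors to its BP_SecuritronPilot controller's StartleTo.
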(event Custom|ScenarioProceedTo
  (params (Actors :type Array%20of%20Actor%20Object%20References))
  (bind _asbp_securitron_pilot (Utilities|Casting|CastToBP_SecuritronPilot (AI|GetAIController 0)))
  (Class|CSecuritronPilot|Startleto _asbp_securitron_pilot Actors))

(event EventBeginPlay
  (bind _outactors (Actor|GetAllActorswithTag "Checkpoint"))
  (bind _returnvalue (Rendering|Material|CreateDynamicMaterialInstance (Variables|Character|GetMesh) 4 "/Game/Dump/General/Enemies/Goomba/skebob_eye_Mat.skebob_eye_Mat" "None" :!class /Script/Engine.PrimitiveComponent))
  (Variables|Default|SetEYEMAT _returnvalue)
  (Variables|Default|SetBBRef (AI|GetBlackboard 0)))

(event Collision|EventActorBeginOverlap
  (params (OtherActor :type Actor%20Object%20Reference)))

(event EventTick
  (params (DeltaSeconds :type Float%20%28single-precision%29))
  (bind _returnvalue (Transformation|GetActorLocation))
  (bind _returnvalue_2 (Utilities|Name|MakeLiteralName "IsTriggered"))
  (bind _returnvalue_3 (Utilities|Name|MakeLiteralName "IsStartled"))
  (bind _bbref (Variables|Default|GetBBRef))
  (bind _returnvalue_4 (ScalableFloat|GetValueasBool _bbref _returnvalue_2))
  (Rendering|Material|SetScalarParameterValue (Variables|Default|GetEYEMAT) _returnvalue_3 (Math|Conversions|ToFloat(Boolean) (ScalableFloat|GetValueasBool _bbref _returnvalue_3)) :!class /Script/Engine.MaterialInstanceDynamic)
  (Rendering|Material|SetScalarParameterValue (Variables|Default|GetEYEMAT) _returnvalue_2 (Math|Conversions|ToFloat(Boolean) _returnvalue_4) :!class /Script/Engine.MaterialInstanceDynamic)
  (if _returnvalue_4
    (if (<= (Variables|Default|GetcurTimer) 0.0)
      (Audio|PlaySoundatLocation "/Game/Dump/General/Audio/SFX/glock_shoot.glock_shoot" (Transformation|GetActorLocation) "0, 0, 0" 1.0 1.0 0.0 0 0 0 0)
      (bind (_outhit _returnvalue_5) (Collision|LineTraceByChannel _returnvalue (+ (+ _returnvalue (* (Math|Vector|GetForwardVector (Math|Rotator|MakeRotfromX (- _returnvalue (Transformation|GetActorLocation (Game|Player|GetPlayerPawn 0))))) -3.2e+03)) (Math|Random|RandomFloatinRange -12.0 12.0)) "TraceTypeQuery3" false (stale EventBeginPlay _outactors) "ForDuration"))
      (if _returnvalue_5
        (Class|CIPlayer|Punch(Message) (.HitActor (Collision|BreakHitResult _outhit)) 3))
      (Variables|Default|SetcurTimer (Math|Random|RandomFloatinRange 0.18 0.28))
      (else
        (Variables|Default|SetcurTimer (- (Variables|Default|GetcurTimer) (Utilities|Time|GetWorldDeltaSeconds)))))))

(fn ConstructionScript)