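; Player Blueprint that grants a starting loadout and delivers in-game email messages to the HUD.
; On BeginPlay, AddItem looks up a glock and a brepsi item in data tables and adds them, plus ammo, to the InventoryComponent.
; After a short delay it sends a garbled "corrupted data" email through SendMessage.
; SendMessage plays a notification sound and passes the message to the first BP_FPS_HUD widget found.
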(event EventBeginPlay
  (InventoryManagement|AddItem)
  (Utilities|FlowControl|Delay 1.0)
  (Class|CIPlayer|SendMessage (Utilities|Struct|MakeEmailItem "adf ,krw2@ re" "djt@hotmail.com" "CORRUPTED_DATA" "hiuhATFHifhudhUYFAGUB%&%&$&%^^E%BNGjkkJ&TH^^&UIKMNJBHGVYT^&*UIIJKNBHVGTYUIKMN BVGFggvbgT&YTFTYUT^&TYhuU*&Y*&^THNKJ97Y&*G^V6f7g8hn*&f6r46drvybU")))

(event Collision|EventActorBeginOverlap
  (params (OtherActor :type Actor%20Object%20Reference)))

(event EventTick
  (params (DeltaSeconds :type Float%20%28single-precision%29)))

(event EventSendMessage
  (params (inMessage :type Email%20Item%20Structure%20%28by%20ref%29))
  (Audio|PlaySound2D "/Game/Dump/General/Audio/SFX/newEmail.newEmail" 1.0 1.0 0.0 0 0)
  (bind _foundwidgets (Widget|GetAllWidgetsOfClass "/Game/Dump/General/UI/BP_FPS_HUD.BP_FPS_HUD_C" true))
  (Default|SendMsg (Utilities|Array|Get(acopy) _foundwidgets) inMessage))

(fn ConstructionScript)